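; BP_Pawn is an input pawn that drives transform operations on the BP_MatrixRepresentative actor, referenced as Chair.
; Each key lazily finds and caches that actor, then Q/W/E (translation), A/S/D and Z/X/C (both commented as rotation) or Space (reset) set its AlterEnum.
; Tab calls its ToggleMajor, Escape quits the game, and the transform logic itself lives outside this pawn.
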(event `GetChair`
  ; get chair reference
  (`self.Chair`
    (:`then`)
    (:`else`
      (bind _returnvalue (`GameplayStatics.GetActorOfClass` "/Game/Blueprints/BP_MatrixRepresentative.BP_MatrixRepresentative_C"))
      (set `self.Chair` _returnvalue))))

(event `Key|SpaceBar`
  (params (Key :type "Key Structure"))
  ; reset
  (:`Pressed`
    (`self.GetChair`)
    (bind _chair (`self.Chair`)
      (:`then`
        (set `/Game/Blueprints/BP_MatrixRepresentative.AlterEnum` "NewEnumerator9" _chair))
      (:`else`))))

(event `Key|Q`
  (params (Key :type "Key Structure"))
  ; Translation
  (:`Pressed`
    (`self.GetChair`)
    (bind _chair (`self.Chair`)
      (:`then`
        (set `/Game/Blueprints/BP_MatrixRepresentative.AlterEnum` "NewEnumerator0" _chair))
      (:`else`))))

(event `Key|W`
  (params (Key :type "Key Structure"))
  ; Translation
  (:`Pressed`
    (`self.GetChair`)
    (bind _chair (`self.Chair`)
      (:`then`
        (set `/Game/Blueprints/BP_MatrixRepresentative.AlterEnum` "NewEnumerator1" _chair))
      (:`else`))))

(event `Key|E`
  (params (Key :type "Key Structure"))
  ; Translation
  (:`Pressed`
    (`self.GetChair`)
    (bind _chair (`self.Chair`)
      (:`then`
        (set `/Game/Blueprints/BP_MatrixRepresentative.AlterEnum` "NewEnumerator2" _chair))
      (:`else`))))

(event `Key|A`
  (params (Key :type "Key Structure"))
  ; Rotate
  (:`Pressed`
    (`self.GetChair`)
    (bind _chair (`self.Chair`)
      (:`then`
        (set `/Game/Blueprints/BP_MatrixRepresentative.AlterEnum` "NewEnumerator3" _chair))
      (:`else`))))

(event `Key|S`
  (params (Key :type "Key Structure"))
  ; Rotate
  (:`Pressed`
    (`self.GetChair`)
    (bind _chair (`self.Chair`)
      (:`then`
        (set `/Game/Blueprints/BP_MatrixRepresentative.AlterEnum` "NewEnumerator4" _chair))
      (:`else`))))

(event `Key|D`
  (params (Key :type "Key Structure"))
  ; Rotate
  (:`Pressed`
    (`self.GetChair`)
    (bind _chair (`self.Chair`)
      (:`then`
        (set `/Game/Blueprints/BP_MatrixRepresentative.AlterEnum` "NewEnumerator5" _chair))
      (:`else`))))

(event `Key|Z`
  (params (Key :type "Key Structure"))
  ; Rotate
  (:`Pressed`
    (`self.GetChair`)
    (bind _chair (`self.Chair`)
      (:`then`
        (set `/Game/Blueprints/BP_MatrixRepresentative.AlterEnum` "NewEnumerator6" _chair))
      (:`else`))))

(event `Key|X`
  (params (Key :type "Key Structure"))
  ; Rotate
  (:`Pressed`
    (`self.GetChair`)
    (bind _chair (`self.Chair`)
      (:`then`
        (set `/Game/Blueprints/BP_MatrixRepresentative.AlterEnum` "NewEnumerator7" _chair))
      (:`else`))))

(event `Key|C`
  (params (Key :type "Key Structure"))
  ; Rotate
  (:`Pressed`
    (`self.GetChair`)
    (bind _chair (`self.Chair`)
      (:`then`
        (set `/Game/Blueprints/BP_MatrixRepresentative.AlterEnum` "NewEnumerator8" _chair))
      (:`else`))))

(event `Key|Tab`
  (params (Key :type "Key Structure"))
  (:`Pressed`
    (`self.GetChair`)
    (bind _chair (`self.Chair`)
      (:`then`
        (`/Game/Blueprints/BP_MatrixRepresentative.ToggleMajor` _chair))
      (:`else`))))

(event `Key|Escape`
  (params (Key :type "Key Structure"))
  (:`Pressed`
    (`KismetSystemLibrary.QuitGame` (`GameplayStatics.GetPlayerController` 0) "Quit")))

(fn `UserConstructionScript`)