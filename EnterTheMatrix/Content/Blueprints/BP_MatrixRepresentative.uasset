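; Demo actor that visualizes a transform matrix by animating a Chair component and showing its values in an on-screen widget, alongside a how-to widget.
; Each tick, AlterEnum selects one axis to translate, rotate or scale over time, then the chair's world transform feeds the matrix widget.
; Mode changes reset the chair unless ManualOverride is set, and Nothing resets it continually.
; ToggleMajor flips the widget's RowMajor flag and resets.
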(event `self.ReceiveBeginPlay`
  (bind _returnvalue (`|CreateWidget` "/Game/Widget/WBP_MatrixDataUI.WBP_MatrixDataUI_C" (`GameplayStatics.GetPlayerController` 0)))
  (`UserWidget.AddToViewport` _returnvalue 0)
  (set `self.MatrixWidget` _returnvalue)
  (bind _returnvalue_2 (`|CreateWidget` "/Game/Widget/WBP_HowTo.WBP_HowTo_C" (`GameplayStatics.GetPlayerController` 0)))
  (`UserWidget.AddToViewport` _returnvalue_2 0))

(event `ResetMatrix`
  (bind _chair (`self.Chair`))
  ; RESET
  (`SceneComponent.K2_SetWorldLocation` _chair (0.0 0.0 0.0) false true)
  (`SceneComponent.K2_SetWorldRotation` :`self` _chair)
  (`SceneComponent.SetWorldScale3D` _chair (1.0 1.0 1.0))
  (`WidgetBlueprintLibrary.SetFocusToGameViewport`))

(event `self.ReceiveTick`
  (params (DeltaSeconds :type "Float (single-precision)"))
  (bind _chair (`self.Chair`))
  (bind _alterenum (`self.AlterEnum`))
  (bind _chair_2 (`self.Chair`))
  (bind (_returnvalue_x _returnvalue_y _returnvalue_z) (`KismetMathLibrary.BreakVector` (`SceneComponent.K2_GetComponentLocation` _chair_2)))
  (bind (_returnvalue_x_2 _returnvalue_y_2 _returnvalue_z_2) (`KismetMathLibrary.BreakVector` (`SceneComponent.K2_GetComponentLocation` _chair_2)))
  (bind (_returnvalue_x_3 _returnvalue_y_3 _returnvalue_z_3) (`KismetMathLibrary.BreakVector` (`SceneComponent.K2_GetComponentLocation` _chair_2)))
  (bind (_returnvalue_roll _returnvalue_pitch _returnvalue_yaw) (`KismetMathLibrary.BreakRotator` (`SceneComponent.K2_GetComponentRotation` (`self.Chair`))))
  (bind (_returnvalue_roll_2 _returnvalue_pitch_2 _returnvalue_yaw_2) (`KismetMathLibrary.BreakRotator` (`SceneComponent.K2_GetComponentRotation` (`self.Chair`))))
  (bind (_returnvalue_roll_3 _returnvalue_pitch_3 _returnvalue_yaw_3) (`KismetMathLibrary.BreakRotator` (`SceneComponent.K2_GetComponentRotation` (`self.Chair`))))
  (bind (_returnvalue_x_4 _returnvalue_y_4 _returnvalue_z_4) (`KismetMathLibrary.BreakVector` (`SceneComponent.K2_GetComponentScale` (`self.Chair`))))
  (bind (_returnvalue_x_5 _returnvalue_y_5 _returnvalue_z_5) (`KismetMathLibrary.BreakVector` (`SceneComponent.K2_GetComponentScale` (`self.Chair`))))
  (bind (_returnvalue_x_6 _returnvalue_y_6 _returnvalue_z_6) (`KismetMathLibrary.BreakVector` (`SceneComponent.K2_GetComponentScale` (`self.Chair`))))
  (if (`|EnumInequality` (`self.CachedEnum`) (`self.AlterEnum`))
    (set `self.CachedEnum` (`self.AlterEnum`))
    (if (not (`self.bManualOverride`))
      (`self.ResetMatrix` :!label _label))
    (else
      (`|ExecutionSequence`
        (:`then_0`
          (set `self.CachedEnum` _alterenum)
          (switch `/Game/E_Alter` _alterenum
            (:`NewEnumerator9`
              (goto _label))
            (:`NewEnumerator0`
              ; Translate
              (`SceneComponent.K2_SetWorldLocation` _chair (`KismetMathLibrary.MakeVector` (+ _returnvalue_x_2 (* (`GameplayStatics.GetWorldDeltaSeconds`) (`self.Speed`))) _returnvalue_y_2 _returnvalue_z_2) false false))
            (:`NewEnumerator1`
              (`SceneComponent.K2_SetWorldLocation` _chair (`KismetMathLibrary.MakeVector` _returnvalue_x_3 (+ _returnvalue_y_3 (* (`GameplayStatics.GetWorldDeltaSeconds`) (`self.Speed`))) _returnvalue_z_3) false false))
            (:`NewEnumerator2`
              (`SceneComponent.K2_SetWorldLocation` _chair (`KismetMathLibrary.MakeVector` _returnvalue_x _returnvalue_y (+ _returnvalue_z (* (`GameplayStatics.GetWorldDeltaSeconds`) (`self.Speed`)))) false false))
            (:`NewEnumerator3`
              ; Rotate
              (`SceneComponent.K2_SetWorldRotation` (`self.Chair`) (`KismetMathLibrary.MakeRotator` (+ _returnvalue_roll_2 (* (`GameplayStatics.GetWorldDeltaSeconds`) (`self.Speed`))) _returnvalue_pitch_2 _returnvalue_yaw_2) false false))
            (:`NewEnumerator4`
              (`SceneComponent.K2_SetWorldRotation` (`self.Chair`) (`KismetMathLibrary.MakeRotator` _returnvalue_roll_3 (+ _returnvalue_pitch_3 (* (`GameplayStatics.GetWorldDeltaSeconds`) (`self.Speed`))) _returnvalue_yaw_3) false false))
            (:`NewEnumerator5`
              (`SceneComponent.K2_SetWorldRotation` (`self.Chair`) (`KismetMathLibrary.MakeRotator` _returnvalue_roll _returnvalue_pitch (+ _returnvalue_yaw (* (`GameplayStatics.GetWorldDeltaSeconds`) (`self.Speed`)))) false false))
            (:`NewEnumerator6`
              ; Scale
              (`SceneComponent.SetWorldScale3D` (`self.Chair`) (`KismetMathLibrary.MakeVector` (+ _returnvalue_x_5 (`GameplayStatics.GetWorldDeltaSeconds`)) _returnvalue_y_5 _returnvalue_z_5)))
            (:`NewEnumerator7`
              (`SceneComponent.SetWorldScale3D` (`self.Chair`) (`KismetMathLibrary.MakeVector` _returnvalue_x_6 (+ _returnvalue_y_6 (`GameplayStatics.GetWorldDeltaSeconds`)) _returnvalue_z_6)))
            (:`NewEnumerator8`
              (`SceneComponent.SetWorldScale3D` (`self.Chair`) (`KismetMathLibrary.MakeVector` _returnvalue_x_4 _returnvalue_y_4 (+ _returnvalue_z_4 (`GameplayStatics.GetWorldDeltaSeconds`)))))))
        (:`then_1`
          (`/Game/Widget/WBP_MatrixDataUI.UpdateValues` (`self.MatrixWidget`) (`SceneComponent.K2_GetComponentToWorld` (`self.Chair`))))))))

(event `ToggleMajor`
  (bind _matrixwidget (`self.MatrixWidget`))
  (set `/Game/Widget/WBP_MatrixDataUI.bRowMajor` (not (`/Game/Widget/WBP_MatrixDataUI.bRowMajor` _matrixwidget)) _matrixwidget)
  (`self.ResetMatrix`))

(fn `UserConstructionScript`)